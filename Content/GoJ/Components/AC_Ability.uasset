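; AC_Ability is a component that manages a Ki resource pool, filled to MaxKi on BeginPlay.
; SpendKi deducts only when enough Ki is available and returns whether it succeeded, while RestoreKi adds Ki without clamping to the maximum.
; Both fire the OnResourceChanged dispatcher when Ki changes, and GetKiPercent returns current Ki as a fraction of the maximum.
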(event EventBeginPlay
  (Variables|Default|SetCurrentKi (Variables|Default|GetMaxKi)))

(event EventTick
  (params (DeltaSeconds :type Float%20%28single-precision%29)))

(fn SpendKi
  (params (Amount :type Float%20%28double-precision%29))
  (if (>= (Variables|Default|GetCurrentKi) Amount)
    (Variables|Default|SetCurrentKi (- (Variables|Default|GetCurrentKi) Amount))
    (Default|CallOnResourceChanged)
    (return true)
    (else
      (return false))))

(fn RestoreKi
  (params (Amount :type Float%20%28double-precision%29))
  (Variables|Default|SetCurrentKi (+ (Variables|Default|GetCurrentKi) Amount))
  (Default|CallOnResourceChanged))

(fn GetKiPercent
  (return (/ (Variables|Default|GetCurrentKi) (Variables|Default|GetMaxKi))))