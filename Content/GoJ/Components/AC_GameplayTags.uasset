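; AC_GameplayTags is an actor component that stores a gameplay tag container, OwnedTags, for its owner.
; It exposes functions to add a tag, remove a tag, read the whole container and test for a tag.
; The HasTag check uses non-exact matching, so querying a parent tag also matches its owned child tags.
; It has no event logic of its own.
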(event EventBeginPlay)

(event EventTick
  (params (DeltaSeconds :type Float%20%28single-precision%29)))

(fn AddTag
  (params (Tag :type Gameplay%20Tag%20Structure))
  (GameplayTags|AddGameplayTag (Variables|Tags|GetOwnedTags) Tag :!class /Script/GameplayTags.BlueprintGameplayTagLibrary))

(fn RemoveTag
  (params (Tag :type Gameplay%20Tag%20Structure))
  (GameplayTags|RemoveGameplayTag (Variables|Tags|GetOwnedTags) Tag :!class /Script/GameplayTags.BlueprintGameplayTagLibrary))

(fn HasTag
  (params (Tag :type Gameplay%20Tag%20Structure))
  (return (GameplayTags|HasAnyTags (Variables|Tags|GetOwnedTags) (GameplayTags|MakeGameplayTagContainerfromTag Tag))))

(fn GetTags
  (return (Variables|Tags|GetOwnedTags)))