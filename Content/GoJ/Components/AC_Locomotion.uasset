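; Actor component that gives its owning Character stamina-limited sprinting, crouching, jumping with an optional double jump, and dodging.
; Request functions update state, with ApplyMovementState setting walk speed by priority of crouch, sprint, then walk.
; Tick drains sprint stamina, stops sprinting when empty, regenerates after a delay and resets the jump count on ground.
; Double jump and dodge use LaunchCharacter, with dodge costing stamina and defaulting to the forward direction.
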(event EventBeginPlay
  (bind _ascharacter (Utilities|Casting|CastToCharacter (Components|GetOwner)))
  (Variables|Locomotion|Runtime|SetOwnerCharacter _ascharacter)
  (bind _ascharacter_movement_component (Utilities|Casting|CastToCharacterMovementComponent (Actor|GetComponentbyClass _ascharacter "/Script/Engine.CharacterMovementComponent")))
  (Variables|Locomotion|Runtime|SetMoveComp _ascharacter_movement_component)
  (Variables|Locomotion|Runtime|SetCurrentStamina (Variables|Locomotion|Stamina|GetMaxStamina)))

(event EventTick
  (params (DeltaSeconds :type Float%20%28single-precision%29))
  (if (Variables|Locomotion|Runtime|GetbIsSprinting)
    (Variables|Locomotion|Runtime|SetCurrentStamina (- (Variables|Locomotion|Runtime|GetCurrentStamina) (* (Variables|Locomotion|Stamina|GetStaminaDrainRate) DeltaSeconds)))
    (Variables|Locomotion|Runtime|SetTimeSinceStaminaUse 0.0)
    (if (<= (Variables|Locomotion|Runtime|GetCurrentStamina) (Math|Float|MakeLiteralFloat 0.0))
      (Variables|Locomotion|Runtime|SetCurrentStamina 0.0)
      (Variables|Locomotion|Runtime|SetbIsSprinting false)
      (CallFunction|ApplyMovementState))
    (else
      (Variables|Locomotion|Runtime|SetTimeSinceStaminaUse (+ (Variables|Locomotion|Runtime|GetTimeSinceStaminaUse) DeltaSeconds))
      (if (and (>= (Variables|Locomotion|Runtime|GetTimeSinceStaminaUse) (Variables|Locomotion|Stamina|GetStaminaRegenDelay)) (< (Variables|Locomotion|Runtime|GetCurrentStamina) (Variables|Locomotion|Stamina|GetMaxStamina)))
        (Variables|Locomotion|Runtime|SetCurrentStamina (+ (Variables|Locomotion|Runtime|GetCurrentStamina) (* (Variables|Locomotion|Stamina|GetStaminaRegenRate) DeltaSeconds))))))
  (if (and (AI|Components|NavMovement|IsMovingonGround (Variables|Locomotion|Runtime|GetMoveComp)) (> (Variables|Locomotion|Runtime|GetJumpCount) (Class|KismetSystemLibrary|MakeLiteralInteger)))
    (Variables|Locomotion|Runtime|SetJumpCount 0)))

(fn RequestSprint
  (params (bWantSprint :type Boolean))
  (Variables|Locomotion|Runtime|SetbIsSprinting (and bWantSprint (and (> (Variables|Locomotion|Runtime|GetCurrentStamina) (Math|Float|MakeLiteralFloat 0.0)) (not (Variables|Locomotion|Runtime|GetbIsCrouched)))))
  (CallFunction|ApplyMovementState))

(fn RequestJump
  (bind _movecomp (Variables|Locomotion|Runtime|GetMoveComp))
  (bind _ownercharacter (Variables|Locomotion|Runtime|GetOwnerCharacter))
  (if (AI|Components|NavMovement|IsMovingonGround _movecomp)
    (Character|Jump _ownercharacter)
    (Variables|Locomotion|Runtime|SetJumpCount 1)
    (elif (and (Variables|Locomotion|Jump|GetbDoubleJumpAllowed) (< (Variables|Locomotion|Runtime|GetJumpCount) (Class|KismetSystemLibrary|MakeLiteralInteger 2)))
      (Character|LaunchCharacter _ownercharacter (Math|Vector|MakeVector 0.0 0.0 (Variables|/Script/Engine.CharacterMovementComponent|GetJumpZVelocity _movecomp)) false true)
      (Variables|Locomotion|Runtime|SetJumpCount (+ (Variables|Locomotion|Runtime|GetJumpCount) (Class|KismetSystemLibrary|MakeLiteralInteger 1))))))

(fn RequestCrouch
  (params (bWantCrouch :type Boolean))
  (bind _ownercharacter (Variables|Locomotion|Runtime|GetOwnerCharacter))
  (Variables|Locomotion|Runtime|SetbIsCrouched bWantCrouch)
  (if bWantCrouch
    (Character|Crouch _ownercharacter)
    (else
      (Character|UnCrouch _ownercharacter)))
  (CallFunction|ApplyMovementState))

(fn RequestDodge
  (params (Direction :type Vector))
  (bind _dodgestaminacost (Variables|Locomotion|Dodge|GetDodgeStaminaCost))
  (bind _ownercharacter (Variables|Locomotion|Runtime|GetOwnerCharacter))
  (if (and (>= (Variables|Locomotion|Runtime|GetCurrentStamina) _dodgestaminacost) (not (Variables|Locomotion|Runtime|GetbIsCrouched)))
    (Variables|Locomotion|Runtime|SetCurrentStamina (- (Variables|Locomotion|Runtime|GetCurrentStamina) _dodgestaminacost))
    (Variables|Locomotion|Runtime|SetTimeSinceStaminaUse 0.0)
    (Character|LaunchCharacter _ownercharacter (* (Math|Vector|Normalize (select (> (Math|Vector|VectorLength Direction) (Math|Float|MakeLiteralFloat 0.1)) Direction (Transformation|GetActorForwardVector _ownercharacter))) (/ (Variables|Locomotion|Dodge|GetDodgeDistance) (Variables|Locomotion|Dodge|GetDodgeDuration))) true false)))

(fn ApplyMovementState
  (Variables|/Script/Engine.CharacterMovementComponent|SetMaxWalkSpeed (Variables|Locomotion|Runtime|GetMoveComp) (select (Variables|Locomotion|Runtime|GetbIsCrouched) (Variables|Locomotion|Speed|GetCrouchSpeed) (select (Variables|Locomotion|Runtime|GetbIsSprinting) (Variables|Locomotion|Speed|GetSprintSpeed) (Variables|Locomotion|Speed|GetWalkSpeed)))))