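; Actor component that gives a Character parkour moves: automatic mantling and an on-demand vault hop.
; Each Tick, a low forward trace detects obstacles, then a downward trace beyond finds the top surface.
; Surfaces above StepUpHeight relative to the estimated feet trigger an instant, unswept teleport onto them, without animation.
; TryParkour separately traces forward at chest height, launches the character upward on a hit, fires OnParkourStarted and returns success.
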(event EventBeginPlay
  (bind _ascharacter (Utilities|Casting|CastToCharacter (Components|GetOwner)))
  (Variables|Default|SetOwnerCharacter _ascharacter)
  (bind _ascharacter_movement_component (Utilities|Casting|CastToCharacterMovementComponent (Actor|GetComponentbyClass _ascharacter "/Script/Engine.CharacterMovementComponent")))
  (Variables|Default|SetMoveComp _ascharacter_movement_component))

(event EventTick
  (params (DeltaSeconds :type Float%20%28single-precision%29))
  (bind _returnvalue (Components|GetOwner))
  (bind _returnvalue_2 (Math|Vector|MakeVector 0.0 0.0 -3e+01))
  (bind _returnvalue_3 (Math|Float|MakeLiteralFloat 3e+01))
  (bind _forwardtracedistance (Variables|Default|GetForwardTraceDistance))
  (bind _mantlemaxheight (Variables|Default|GetMantleMaxHeight))
  (bind _returnvalue_4 (Transformation|GetActorLocation _returnvalue))
  (bind _returnvalue_5 (Transformation|GetActorForwardVector _returnvalue))
  (bind _returnvalue_6 (Math|Vector|MakeVector 0.0 0.0 _mantlemaxheight))
  (bind _returnvalue_7 (+ _forwardtracedistance _returnvalue_3))
  (bind _returnvalue_8 (+ _returnvalue_4 _returnvalue_2))
  (bind _returnvalue_9 (* _returnvalue_5 _returnvalue_7))
  (bind _returnvalue_10 (+ _returnvalue_4 _returnvalue_9))
  (bind _returnvalue_11 (+ _returnvalue_10 _returnvalue_6))
  (bind _returnvalue_12 (Collision|LineTraceByChannel _returnvalue_8 (+ _returnvalue_8 (* _returnvalue_5 (Variables|Default|GetForwardTraceDistance))) "TraceTypeQuery1" false 0 "None"))
  (if _returnvalue_12
    (bind (_outhit _returnvalue_13) (Collision|LineTraceByChannel _returnvalue_11 (+ _returnvalue_11 (Math|Vector|MakeVector 0.0 0.0 -3e+02)) "TraceTypeQuery1" false 0 "None"))
    (if _returnvalue_13
      (if (> (- (.Z (Math|Vector|BreakVector (.ImpactPoint (Collision|BreakHitResult _outhit)))) (- (.Z (Math|Vector|BreakVector _returnvalue_4)) (Math|Float|MakeLiteralFloat 88.0))) (Variables|Default|GetStepUpHeight))
        (Transformation|SetActorLocation _returnvalue (+ (.ImpactPoint (Collision|BreakHitResult _outhit)) (Math|Vector|MakeVector 0.0 0.0 9e+01)) false false)))))

(fn TryParkour
  (bind _returnvalue (Math|Vector|MakeVector 0.0 0.0 5e+01))
  (bind _ownercharacter (Variables|Default|GetOwnerCharacter))
  (bind _returnvalue_2 (Transformation|GetActorLocation _ownercharacter))
  (bind _returnvalue_3 (+ _returnvalue_2 _returnvalue))
  (bind _returnvalue_4 (Collision|LineTraceByChannel _returnvalue_3 (+ _returnvalue_3 (* (Transformation|GetActorForwardVector _ownercharacter) (Variables|Default|GetForwardTraceDistance))) "TraceTypeQuery1" false 0 "None"))
  (if _returnvalue_4
    (Character|LaunchCharacter _ownercharacter (Math|Vector|MakeVector 0.0 0.0 6e+02) false true)
    (Default|CallOnParkourStarted)
    (return true)
    (else
      (return false))))