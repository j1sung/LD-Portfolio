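; AC_Combat is an actor component that deals melee damage to actors carrying an AC_Health component.
; Melee, light and heavy attack functions damage a supplied target, heavy at double AttackDamage, then fire OnHitLanded.
; AttackForward instead sphere-traces for pawns ahead of the owner up to AttackRange and damages the hit actor without firing OnHitLanded.
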(event EventBeginPlay)

(event EventTick
  (params (DeltaSeconds :type Float%20%28single-precision%29)))

(fn MeleeAttack0
  (params (Target :type Actor%20Object%20Reference))
  (bind _asac_health (Utilities|Casting|CastToAC_Health (Actor|GetComponentbyClass Target "/Game/GoJ/Components/AC_Health.AC_Health_C")))
  (Default|ReceiveDamage _asac_health (Variables|Default|GetAttackDamage))
  (Default|CallOnHitLanded))

(fn LightAttack
  (params (Target :type Actor%20Object%20Reference))
  (bind _asac_health (Utilities|Casting|CastToAC_Health (Actor|GetComponentbyClass Target "/Game/GoJ/Components/AC_Health.AC_Health_C")))
  (Default|ReceiveDamage _asac_health (Variables|Default|GetAttackDamage))
  (Default|CallOnHitLanded))

(fn HeavyAttack
  (params (Target :type Actor%20Object%20Reference))
  (bind _asac_health (Utilities|Casting|CastToAC_Health (Actor|GetComponentbyClass Target "/Game/GoJ/Components/AC_Health.AC_Health_C")))
  (Default|ReceiveDamage _asac_health (* (Variables|Default|GetAttackDamage) (Math|Float|MakeLiteralFloat 2.0)))
  (Default|CallOnHitLanded))

(fn AttackForward
  (bind _returnvalue (Components|GetOwner))
  (bind _returnvalue_2 (Math|Vector|MakeVector 0.0 0.0 5e+01))
  (bind _returnvalue_3 (Transformation|GetActorLocation _returnvalue))
  (bind _returnvalue_4 (+ _returnvalue_3 _returnvalue_2))
  (bind (_outhit _returnvalue_5) (Collision|SphereTraceForObjects _returnvalue_4 (+ _returnvalue_4 (* (Transformation|GetActorForwardVector (Components|GetOwner)) (Variables|Default|GetAttackRange))) 45.0 (Utilities|Array|MakeArray (Utilities|Enum|LiteralenumEObjectTypeQuery "ObjectTypeQuery3")) false 0 "None"))
  (if _returnvalue_5
    (bind _asac_health (Utilities|Casting|CastToAC_Health (Actor|GetComponentbyClass (.HitActor (Collision|BreakHitResult _outhit)) "/Game/GoJ/Components/AC_Health.AC_Health_C")))
    (Default|ReceiveDamage _asac_health (Variables|Default|GetAttackDamage))))