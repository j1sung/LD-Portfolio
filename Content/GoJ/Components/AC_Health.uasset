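; AC_Health is a health component that tracks current and maximum health and death state for its owner.
; BeginPlay fills health to max, and ReceiveDamage and Heal adjust it while alive, broadcasting OnHealthChanged.
; At zero or below, damage sets the dead flag and fires OnDeath; the change event fires before health clamps to zero.
; Heal has no upper clamp, and helper functions report health fraction and alive state.
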(event EventBeginPlay
  (Variables|Default|SetCurrentHealth (Variables|Default|GetMaxHealth)))

(event EventTick
  (params (DeltaSeconds :type Float%20%28single-precision%29)))

(fn Heal
  (params (Amount :type Float%20%28double-precision%29))
  (if (not (Variables|Default|GetbIsDead))
    (Variables|Default|SetCurrentHealth (+ (Variables|Default|GetCurrentHealth) Amount))
    (Default|CallOnHealthChanged)))

(fn GetHealthPercent
  (return (/ (Variables|Default|GetCurrentHealth) (Variables|Default|GetMaxHealth))))

(fn IsAlive
  (return (not (Variables|Default|GetbIsDead))))

(fn ReceiveDamage
  (params (Amount :type Float%20%28double-precision%29))
  (if (not (Variables|Default|GetbIsDead))
    (Variables|Default|SetCurrentHealth (- (Variables|Default|GetCurrentHealth) Amount))
    (Default|CallOnHealthChanged)
    (if (<= (Variables|Default|GetCurrentHealth) (Math|Float|MakeLiteralFloat 0.0))
      (Variables|Default|SetCurrentHealth 0.0)
      (Variables|Default|SetbIsDead true)
      (Default|CallOnDeath))))