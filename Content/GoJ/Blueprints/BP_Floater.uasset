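; BP_Floater is a platform actor that eases back and forth between its placed transform and an offset set by its FloatTarget component, with optional continuous spin.
; Tick advances a phase from TravelTime, starting at PhaseOffset, and a cosine curve blends location (unrotated world-space offset), rotation and scale.
; Rotation interpolates forward and up vectors, then applies SpinYawRate around world Z.
; The construction script assigns Mesh; older unconnected movement chains remain unused.
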(event EventBeginPlay
  (bind _self self)
  (Variables|Default|SetBaseLoc (Transformation|GetActorLocation _self))
  (Variables|Default|SetBaseRot (Transformation|GetActorRotation _self))
  (Variables|Default|SetBaseScale (Transformation|GetActorScale3D _self))
  (Variables|Default|SetPhase (Variables|Float|GetPhaseOffset)))

(event Collision|EventActorBeginOverlap
  (params (OtherActor :type Actor%20Object%20Reference)))

(event EventTick
  (params (DeltaSeconds :type Float%20%28single-precision%29))
  (bind _self self)
  (bind _baserot (Variables|Default|GetBaseRot))
  (bind _floattarget (Variables|Default|GetFloatTarget))
  (bind _baserot_2 (Variables|Default|GetBaseRot))
  (bind _baserot_3 (Variables|Default|GetBaseRot))
  (bind _returnvalue (Math|Vector|GetForwardVector _baserot_2))
  (bind _returnvalue_2 (Math|Vector|GetUpVector _baserot_3))
  (bind _relativerotation (Variables|/Script/Engine.SceneComponent|GetRelativeRotation _floattarget))
  (bind _returnvalue_3 (Math|Rotator|CombineRotators _baserot _relativerotation))
  (Variables|Default|SetPhase (+ (Variables|Default|GetPhase) (/ DeltaSeconds (+ (* (Variables|Float|GetTravelTime) (Math|Float|MakeLiteralFloat 2.0)) (Math|Float|MakeLiteralFloat 0.001)))))
  (Variables|Default|SetSpinAngle (+ (Variables|Default|GetSpinAngle) (* (Variables|Float|GetSpinYawRate) DeltaSeconds)))
  (Transformation|SetActorLocation _self (+ (Variables|Default|GetBaseLoc) (* (Variables|/Script/Engine.SceneComponent|GetRelativeLocation (Variables|Default|GetFloatTarget)) (- (Math|Float|MakeLiteralFloat 0.5) (* (Math|Float|MakeLiteralFloat 0.5) (Math|Trig|Cos(Degrees) (* (Variables|Default|GetPhase) (Math|Float|MakeLiteralFloat 3.6e+02))))))) false false)
  (Transformation|SetActorRotation _self (Math|Rotator|MakeRotfromXZ (Math|Vector|MakeVector (- (* (.X (Math|Vector|BreakVector (+ _returnvalue (* (- (Math|Vector|GetForwardVector _returnvalue_3) _returnvalue) (- (Math|Float|MakeLiteralFloat 0.5) (* (Math|Float|MakeLiteralFloat 0.5) (Math|Trig|Cos(Degrees) (* (Variables|Default|GetPhase) (Math|Float|MakeLiteralFloat 3.6e+02))))))))) (Math|Trig|Cos(Degrees) (Variables|Default|GetSpinAngle))) (* (.Y (Math|Vector|BreakVector (+ _returnvalue (* (- (Math|Vector|GetForwardVector _returnvalue_3) _returnvalue) (- (Math|Float|MakeLiteralFloat 0.5) (* (Math|Float|MakeLiteralFloat 0.5) (Math|Trig|Cos(Degrees) (* (Variables|Default|GetPhase) (Math|Float|MakeLiteralFloat 3.6e+02))))))))) (Math|Trig|Sin(Degrees) (Variables|Default|GetSpinAngle)))) (+ (* (.X (Math|Vector|BreakVector (+ _returnvalue (* (- (Math|Vector|GetForwardVector _returnvalue_3) _returnvalue) (- (Math|Float|MakeLiteralFloat 0.5) (* (Math|Float|MakeLiteralFloat 0.5) (Math|Trig|Cos(Degrees) (* (Variables|Default|GetPhase) (Math|Float|MakeLiteralFloat 3.6e+02))))))))) (Math|Trig|Sin(Degrees) (Variables|Default|GetSpinAngle))) (* (.Y (Math|Vector|BreakVector (+ _returnvalue (* (- (Math|Vector|GetForwardVector _returnvalue_3) _returnvalue) (- (Math|Float|MakeLiteralFloat 0.5) (* (Math|Float|MakeLiteralFloat 0.5) (Math|Trig|Cos(Degrees) (* (Variables|Default|GetPhase) (Math|Float|MakeLiteralFloat 3.6e+02))))))))) (Math|Trig|Cos(Degrees) (Variables|Default|GetSpinAngle)))) (.Z (Math|Vector|BreakVector (+ _returnvalue (* (- (Math|Vector|GetForwardVector _returnvalue_3) _returnvalue) (- (Math|Float|MakeLiteralFloat 0.5) (* (Math|Float|MakeLiteralFloat 0.5) (Math|Trig|Cos(Degrees) (* (Variables|Default|GetPhase) (Math|Float|MakeLiteralFloat 3.6e+02)))))))))) (Math|Vector|MakeVector (- (* (.X (Math|Vector|BreakVector (+ _returnvalue_2 (* (- (Math|Vector|GetUpVector _returnvalue_3) _returnvalue_2) (- (Math|Float|MakeLiteralFloat 0.5) (* (Math|Float|MakeLiteralFloat 0.5) (Math|Trig|Cos(Degrees) (* (Variables|Default|GetPhase) (Math|Float|MakeLiteralFloat 3.6e+02))))))))) (Math|Trig|Cos(Degrees) (Variables|Default|GetSpinAngle))) (* (.Y (Math|Vector|BreakVector (+ _returnvalue_2 (* (- (Math|Vector|GetUpVector _returnvalue_3) _returnvalue_2) (- (Math|Float|MakeLiteralFloat 0.5) (* (Math|Float|MakeLiteralFloat 0.5) (Math|Trig|Cos(Degrees) (* (Variables|Default|GetPhase) (Math|Float|MakeLiteralFloat 3.6e+02))))))))) (Math|Trig|Sin(Degrees) (Variables|Default|GetSpinAngle)))) (+ (* (.X (Math|Vector|BreakVector (+ _returnvalue_2 (* (- (Math|Vector|GetUpVector _returnvalue_3) _returnvalue_2) (- (Math|Float|MakeLiteralFloat 0.5) (* (Math|Float|MakeLiteralFloat 0.5) (Math|Trig|Cos(Degrees) (* (Variables|Default|GetPhase) (Math|Float|MakeLiteralFloat 3.6e+02))))))))) (Math|Trig|Sin(Degrees) (Variables|Default|GetSpinAngle))) (* (.Y (Math|Vector|BreakVector (+ _returnvalue_2 (* (- (Math|Vector|GetUpVector _returnvalue_3) _returnvalue_2) (- (Math|Float|MakeLiteralFloat 0.5) (* (Math|Float|MakeLiteralFloat 0.5) (Math|Trig|Cos(Degrees) (* (Variables|Default|GetPhase) (Math|Float|MakeLiteralFloat 3.6e+02))))))))) (Math|Trig|Cos(Degrees) (Variables|Default|GetSpinAngle)))) (.Z (Math|Vector|BreakVector (+ _returnvalue_2 (* (- (Math|Vector|GetUpVector _returnvalue_3) _returnvalue_2) (- (Math|Float|MakeLiteralFloat 0.5) (* (Math|Float|MakeLiteralFloat 0.5) (Math|Trig|Cos(Degrees) (* (Variables|Default|GetPhase) (Math|Float|MakeLiteralFloat 3.6e+02))))))))))))
  (Transformation|SetActorScale3D _self (+ (Variables|Default|GetBaseScale) (* (- (* (Variables|Default|GetBaseScale) (Variables|/Script/Engine.SceneComponent|GetRelativeScale3D (Variables|Default|GetFloatTarget))) (Variables|Default|GetBaseScale)) (- (Math|Float|MakeLiteralFloat 0.5) (* (Math|Float|MakeLiteralFloat 0.5) (Math|Trig|Cos(Degrees) (* (Variables|Default|GetPhase) (Math|Float|MakeLiteralFloat 3.6e+02)))))))))

(fn ConstructionScript
  (Components|StaticMesh|SetStaticMesh (Variables|Default|GetPlatformMesh) (Variables|Float|GetMesh)))