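; BP_WindColumn is an interactable wind column that, once activated, launches overlapping characters up to a target point.
; HandleInteract activates it, and Tick fades in the child BP_SpiritVent.
; An overlapping character is frozen for a hold time, then a camera shake fires and constant-speed interpolation moves it, unswept, to LaunchTarget before restoring Falling movement.
; The construction script sets the target's height from LaunchHeight.
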(event EventBeginPlay
  (Collision|SetCollisionResponsetoChannel (Variables|Default|GetTriggerVolume) "ECC_Visibility" "ECR_Block")
  (CallFunction|ApplyVentAlpha self 0.0))

(event Collision|EventActorBeginOverlap
  (params (OtherActor :type Actor%20Object%20Reference))
  (if (and (Variables|Default|GetbActive) (not (or (Variables|Default|GetbHolding) (Variables|Default|GetbLaunching))))
    (bind _ascharacter (Utilities|Casting|CastToCharacter OtherActor))
    (Variables|Default|SetRider _ascharacter)
    (Variables|Default|SetTargetLoc (Transformation|GetWorldLocation (Variables|Default|GetLaunchTarget)))
    (Variables|Default|SetHoldRemaining (Variables|Default|GetHoldDuration))
    (Variables|Default|SetbHolding true)
    (Pawn|Components|CharacterMovement|SetMovementMode (Variables|/Script/Engine.Character|GetCharacterMovement _ascharacter) "MOVE_None" 0)))

(event EventTick
  (params (DeltaSeconds :type Float%20%28single-precision%29))
  (bind _returnvalue (Game|GetPlayerController 0))
  (bind _self self)
  (bind _rider (Variables|Default|GetRider))
  (bind _targetloc (Variables|Default|GetTargetLoc))
  (bind _launchspeed (Variables|Default|GetLaunchSpeed))
  (bind _returnvalue_2 (Transformation|GetActorLocation _rider))
  (bind _returnvalue_3 (Math|Interpolation|VInterptoConstant _returnvalue_2 _targetloc DeltaSeconds _launchspeed))
  (if (not (Variables|Default|GetbActive))
    (CallFunction|ApplyVentAlpha _self 0.0)
    (else
      (CallFunction|UpdateFade _self DeltaSeconds)
      (if (Variables|Default|GetbHolding)
        (Variables|Default|SetHoldRemaining (- (Variables|Default|GetHoldRemaining) DeltaSeconds))
        (if (<= (- (Variables|Default|GetHoldRemaining) DeltaSeconds) (Math|Float|MakeLiteralFloat 0.0))
          (Variables|Default|SetbHolding false)
          (Variables|Default|SetbLaunching true)
          (Utilities|IsValid _returnvalue
            (:Is%20Valid
              (Game|Feedback|ClientStartCameraShake _returnvalue "/Game/GoJ/Interactables/BP_DoorCamShake.BP_DoorCamShake_C" (Variables|Default|GetShakeScale) "CameraLocal" "0, 0, 0"))))
        (elif (Variables|Default|GetbLaunching)
          (Transformation|SetActorLocation _rider _returnvalue_3 false false)
          (if (< (Math|Vector|Distance(Vector) _returnvalue_3 _targetloc) (Math|Float|MakeLiteralFloat 5.0))
            (Transformation|SetActorLocation _rider _targetloc false false)
            (Pawn|Components|CharacterMovement|SetMovementMode (Variables|/Script/Engine.Character|GetCharacterMovement _rider) "MOVE_Falling" 0)
            (Variables|Default|SetbLaunching false)))))))

(event EventHandleInteract
  (if (not (Variables|Default|GetbActive))
    (Variables|Default|SetFadeElapsed 0.0)
    (Variables|Default|SetbActive true)))

(fn ConstructionScript
  (bind _launchtarget (Variables|Default|GetLaunchTarget))
  (bind _relativelocation (Variables|/Script/Engine.SceneComponent|GetRelativeLocation _launchtarget))
  (Transformation|SetRelativeLocation _launchtarget (Math|Vector|MakeVector (.X (Math|Vector|BreakVector _relativelocation)) (.Y (Math|Vector|BreakVector _relativelocation)) (Variables|Default|GetLaunchHeight)) false false))

(fn ApplyVentAlpha
  (params (Alpha :type Float%20%28double-precision%29))
  (bind _asbp_spirit_vent (Utilities|Casting|CastToBP_SpiritVent (Variables|/Script/Engine.ChildActorComponent|GetChildActor (Variables|Default|GetBP_SpiritVent))))
  (Default|SetFadeAlpha _asbp_spirit_vent Alpha))

(fn UpdateFade
  (params (DeltaSeconds :type Float%20%28double-precision%29))
  (bind _fadeinduration (Variables|Default|GetFadeInDuration))
  (if (<= (Variables|Default|GetFadeElapsed) _fadeinduration)
    (Variables|Default|SetFadeElapsed (+ (Variables|Default|GetFadeElapsed) DeltaSeconds))
    (CallFunction|ApplyVentAlpha self (select (> (/ (+ (Variables|Default|GetFadeElapsed) DeltaSeconds) (select (> _fadeinduration (Math|Float|MakeLiteralFloat 0.0001)) _fadeinduration (Math|Float|MakeLiteralFloat 0.0001))) (Math|Float|MakeLiteralFloat 1.0)) (Math|Float|MakeLiteralFloat 1.0) (/ (+ (Variables|Default|GetFadeElapsed) DeltaSeconds) (select (> _fadeinduration (Math|Float|MakeLiteralFloat 0.0001)) _fadeinduration (Math|Float|MakeLiteralFloat 0.0001)))))))