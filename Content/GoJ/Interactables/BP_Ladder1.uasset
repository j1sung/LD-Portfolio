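; Interactable ladder that automatically carries the player character up to its top.
; HandleInteract stores the player, sets a target ClimbHeight up and slightly along the ladder's forward vector, and disables character movement.
; Tick moves the climber there at constant ClimbSpeed without sweeping, then snaps to the target and restores Walking.
; SetLadderOccupied stores an occupancy flag and broadcasts OnLadderOccupied, but the climb logic never calls it.
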(event EventBeginPlay)

(event Collision|EventActorBeginOverlap
  (params (OtherActor :type Actor%20Object%20Reference)))

(event EventTick
  (params (DeltaSeconds :type Float%20%28single-precision%29))
  (bind _climber (Variables|Default|GetClimber))
  (bind _climbtarget (Variables|Default|GetClimbTarget))
  (bind _climbspeed (Variables|Ladder|GetClimbSpeed))
  (bind _returnvalue (Transformation|GetActorLocation _climber))
  (bind _returnvalue_2 (Math|Interpolation|VInterptoConstant _returnvalue _climbtarget DeltaSeconds _climbspeed))
  (if (Variables|Default|GetbClimbing)
    (Transformation|SetActorLocation _climber _returnvalue_2 false false)
    (if (< (Math|Vector|Distance(Vector) _returnvalue_2 _climbtarget) (Math|Float|MakeLiteralFloat 5.0))
      (Transformation|SetActorLocation _climber _climbtarget false false)
      (Pawn|Components|CharacterMovement|SetMovementMode (Variables|/Script/Engine.Character|GetCharacterMovement _climber) "MOVE_Walking" 0)
      (Variables|Default|SetbClimbing false))))

(event EventHandleInteract
  (if (not (Variables|Default|GetbClimbing))
    (bind _ascharacter (Utilities|Casting|CastToCharacter (Game|Player|GetPlayerPawn 0)))
    (Variables|Default|SetClimber _ascharacter)
    (Variables|Default|SetClimbTarget (+ (Transformation|GetActorLocation _ascharacter) (+ (Math|Vector|MakeVector 0.0 0.0 (Variables|Ladder|GetClimbHeight)) (* (Transformation|GetActorForwardVector self) (Math|Float|MakeLiteralFloat 6e+01)))))
    (Pawn|Components|CharacterMovement|SetMovementMode (Variables|/Script/Engine.Character|GetCharacterMovement _ascharacter) "MOVE_None" 0)
    (Variables|Default|SetbClimbing true)))

(fn ConstructionScript)

(fn SetLadderOccupied
  (params (bWantOccupy :type Boolean))
  (Variables|Default|SetbOccupied bWantOccupy)
  (Default|CallOnLadderOccupied))