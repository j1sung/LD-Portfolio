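; Chimney passage interactable that carries an overlapping character along a spline, one way from start to end.
; Overlap disables the character's movement and starts a camera shake; the construction script pins the entry trigger to the first spline point.
; Tick advances the rider at constant speed, yawing the body and smoothly steering control rotation along the spline.
; At the end, the rider switches to falling and is launched along the spline direction at travel speed.
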(event Collision|EventActorBeginOverlap
  (params (OtherActor :type Actor%20Object%20Reference))
  (bind _returnvalue (Game|GetPlayerController 0))
  (if (not (Variables|Default|GetbTraversing))
    (bind _ascharacter (Utilities|Casting|CastToCharacter OtherActor))
    (Variables|Default|SetRider _ascharacter)
    (Variables|Default|SetDistanceAlong 0.0)
    (Variables|Default|SetbTraversing true)
    (Pawn|Components|CharacterMovement|SetMovementMode (Variables|/Script/Engine.Character|GetCharacterMovement _ascharacter) "MOVE_None" 0)
    (Utilities|IsValid _returnvalue
      (:Is%20Valid
        (Game|Feedback|ClientStartCameraShake _returnvalue "/Game/GoJ/Interactables/BP_DoorCamShake.BP_DoorCamShake_C" (Variables|Default|GetShakeScale) "CameraLocal" "0, 0, 0")))))

(event EventTick
  (params (DeltaSeconds :type Float%20%28single-precision%29))
  (bind _rider (Variables|Default|GetRider))
  (bind _splinepath (Variables|Default|GetSplinePath))
  (bind _returnvalue (Pawn|GetController _rider))
  (bind _charactermovement (Variables|/Script/Engine.Character|GetCharacterMovement _rider))
  (if (Variables|Default|GetbTraversing)
    (Variables|Default|SetDistanceAlong (+ (Variables|Default|GetDistanceAlong) (* (Variables|Default|GetTravelSpeed) DeltaSeconds)))
    (Transformation|SetActorRotation _rider (Math|Rotator|MakeRotator 0.0 0.0 (.Yaw (Math|Rotator|BreakRotator (Math|Rotator|MakeRotfromX (Spline|GetDirectionatDistanceAlongSpline _splinepath (+ (Variables|Default|GetDistanceAlong) (* (Variables|Default|GetTravelSpeed) DeltaSeconds)) "World"))))))
    (Pawn|SetControlRotation _returnvalue (Math|Interpolation|RInterpTo (Pawn|GetControlRotation _returnvalue :!class /Script/Engine.Controller) (Math|Rotator|MakeRotfromX (Spline|GetDirectionatDistanceAlongSpline _splinepath (+ (Variables|Default|GetDistanceAlong) (* (Variables|Default|GetTravelSpeed) DeltaSeconds)) "World")) DeltaSeconds 4.0))
    (if (>= (+ (Variables|Default|GetDistanceAlong) (* (Variables|Default|GetTravelSpeed) DeltaSeconds)) (Spline|GetSplineLength _splinepath))
      (Transformation|SetActorLocation _rider (Spline|GetLocationatDistanceAlongSpline _splinepath (Spline|GetSplineLength _splinepath) "World") false false)
      (Pawn|Components|CharacterMovement|SetMovementMode _charactermovement "MOVE_Falling" 0)
      (Variables|/Script/Engine.MovementComponent|SetVelocity _charactermovement (* (Spline|GetDirectionatDistanceAlongSpline _splinepath (+ (Variables|Default|GetDistanceAlong) (* (Variables|Default|GetTravelSpeed) DeltaSeconds)) "World") (Variables|Default|GetTravelSpeed)))
      (Variables|Default|SetbTraversing false)
      (else
        (Transformation|SetActorLocation _rider (Spline|GetLocationatDistanceAlongSpline _splinepath (+ (Variables|Default|GetDistanceAlong) (* (Variables|Default|GetTravelSpeed) DeltaSeconds)) "World") false false)))))

(fn ConstructionScript
  (Transformation|SetRelativeLocation (Variables|Default|GetEntryTrigger) (Spline|GetLocationatSplinePoint (Variables|Default|GetSplinePath) 0 "Local") false false))