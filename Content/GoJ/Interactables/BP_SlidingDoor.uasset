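; Sliding door actor that moves when a Character overlaps it, opening by default or closing if set to start open.
; Leaving reverses the motion, unless the Once option latches it after the first trigger.
; Tick advances an alpha over the slide duration, smoothstep-eases the mesh offset, and shakes the first player's camera when movement leaves or reaches either end.
; The construction script applies configurable mesh, scale and material.
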(event EventBeginPlay
  (Variables|Default|SetClosedLoc (Variables|/Script/Engine.SceneComponent|GetRelativeLocation (Variables|Default|GetDoorMesh)))
  (if (Variables|Default|GetbStartOpen)
    (Variables|Default|SetAlpha 1.0)
    (Variables|Default|SetbOpening true)))

(event Collision|EventActorBeginOverlap
  (params (OtherActor :type Actor%20Object%20Reference))
  (if (not (Variables|Default|GetbLatched))
    (Utilities|Casting|CastToCharacter OtherActor)
    (Variables|Default|SetbOpening (not (Variables|Default|GetbStartOpen)))
    (if (Variables|Default|GetbOnce)
      (Variables|Default|SetbLatched true))))

(event Collision|EventActorEndOverlap
  (params (OtherActor :type Actor%20Object%20Reference))
  (if (not (Variables|Default|GetbLatched))
    (Utilities|Casting|CastToCharacter OtherActor)
    (Variables|Default|SetbOpening (Variables|Default|GetbStartOpen))))

(event EventTick
  (params (DeltaSeconds :type Float%20%28single-precision%29))
  (bind _returnvalue (Game|GetPlayerController 0))
  (bind _slideduration (Variables|Default|GetSlideDuration))
  (bind _returnvalue_2 (Math|Float|Max(Float) _slideduration 0.01))
  (bind _returnvalue_3 (/ DeltaSeconds _returnvalue_2))
  (Variables|Default|SetPrevAlpha (Variables|Default|GetAlpha))
  (Variables|Default|SetAlpha (Math|Float|Clamp(Float) (+ (Variables|Default|GetPrevAlpha) (select (Variables|Default|GetbOpening) _returnvalue_3 (- 0.0 _returnvalue_3)))))
  (Transformation|SetRelativeLocation (Variables|Default|GetDoorMesh) (+ (Variables|Default|GetClosedLoc) (* (Variables|Default|GetSlideOffset) (* (* (Variables|Default|GetAlpha) (Variables|Default|GetAlpha)) (- (Math|Float|MakeLiteralFloat 3.0) (* (Math|Float|MakeLiteralFloat 2.0) (Variables|Default|GetAlpha)))))) false false)
  (if (and (!= (Variables|Default|GetAlpha) (Variables|Default|GetPrevAlpha)) (or (or (>= (Variables|Default|GetAlpha) (Math|Float|MakeLiteralFloat 1.0)) (<= (Variables|Default|GetAlpha) (Math|Float|MakeLiteralFloat 0.0))) (or (>= (Variables|Default|GetPrevAlpha) 1.0) (<= (Variables|Default|GetPrevAlpha) 0.0))))
    (Utilities|IsValid _returnvalue
      (:Is%20Valid
        (Game|Feedback|ClientStartCameraShake _returnvalue "/Game/GoJ/Interactables/BP_DoorCamShake.BP_DoorCamShake_C" (Variables|Default|GetShakeScale) "CameraLocal" "0, 0, 0")))))

(fn ConstructionScript
  (Transformation|SetRelativeScale3D (Variables|Default|GetDoorMesh) (Variables|Default|GetDoorScale))
  (Components|StaticMesh|SetStaticMesh (Variables|Default|GetDoorMesh) (Variables|Default|GetDoorMeshAsset))
  (Utilities|IsValid (Variables|Default|GetDoorMaterial)
    (:Is%20Valid
      (Rendering|Material|SetMaterial (Variables|Default|GetDoorMesh) 0 (Variables|Default|GetDoorMaterial)))))