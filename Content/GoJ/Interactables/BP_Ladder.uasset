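; Interactable ladder that carries player 0's pawn up and over the top when HandleInteract fires.
; Mover pawns switch to Flying and run two delay-sequenced linear-velocity layered moves, up then forward, before Falling, while toggling LadderClimbing on the sandbox animation Blueprint.
; Pawns without a Mover fall back to Character: movement is disabled and Tick interpolates straight to the exit point, then restores Walking.
; SetLadderOccupied is separate from the climb flow.
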(event EventBeginPlay)

(event Collision|EventActorBeginOverlap
  (params (OtherActor :type Actor%20Object%20Reference)))

(event EventTick
  (params (DeltaSeconds :type Float%20%28single-precision%29))
  (bind _climbtarget (Variables|Default|GetClimbTarget))
  (if (Variables|Default|GetbClimbing)
    (bind _ascharacter (Utilities|Casting|CastToCharacter (Variables|Default|GetClimber)))
    (Transformation|SetActorLocation _ascharacter (Math|Interpolation|VInterptoConstant (Transformation|GetActorLocation _ascharacter) _climbtarget DeltaSeconds (Variables|Ladder|GetClimbSpeed)) false false)
    (if (< (Math|Vector|Distance(Vector) (Math|Interpolation|VInterptoConstant (Transformation|GetActorLocation _ascharacter) _climbtarget DeltaSeconds (Variables|Ladder|GetClimbSpeed)) _climbtarget) (Math|Float|MakeLiteralFloat 5.0))
      (Transformation|SetActorLocation _ascharacter _climbtarget false false)
      (Pawn|Components|CharacterMovement|SetMovementMode (Variables|/Script/Engine.Character|GetCharacterMovement _ascharacter) "MOVE_Walking" 0)
      (Variables|Default|SetbClimbing false))))

(event EventHandleInteract
  (bind _returnvalue (Game|Player|GetPlayerPawn 0))
  (bind _self self)
  (bind _returnvalue_2 (Transformation|GetActorLocation _self))
  (bind (_x _y) (Math|Vector|BreakVector _returnvalue_2))
  (if (not (Variables|Default|GetbClimbing))
    (Utilities|IsValid _returnvalue
      (:Is%20Valid
        (Variables|Default|SetClimber _returnvalue)
        (Variables|Default|SetClimbTarget (+ (Transformation|GetActorLocation _returnvalue) (Math|Vector|MakeVector 0.0 0.0 (+ (Variables|Ladder|GetClimbHeight) (Variables|Ladder|GetClimbTopClearance)))))
        (Variables|Default|SetClimbExitTarget (+ (Math|Vector|MakeVector _x _y (.Z (Math|Vector|BreakVector (Variables|Default|GetClimbTarget)))) (* (Class|KismetMathLibrary|VectorNormal2D (- (Transformation|GetActorLocation _self) (Transformation|GetActorLocation _returnvalue)) 0.0001) (Variables|Ladder|GetClimbExitDistance))))
        (bind _asmover_component (Utilities|Casting|CastToMoverComponent (Actor|GetComponentbyClass _returnvalue "/Script/Mover.MoverComponent"))
          (:then
            (Variables|Default|SetClimberMover _asmover_component)
            (Variables|Default|SetPreClimbMode (Class|MoverComponent|GetMovementModeName _asmover_component))
            (Variables|Default|SetClimbDuration (Math|Float|Max(Float) 0.01 (/ (Math|Vector|Distance(Vector) (Transformation|GetActorLocation _returnvalue) (Variables|Default|GetClimbTarget)) (Math|Float|Max(Float) (Variables|Ladder|GetClimbSpeed) 1.0))))
            (Variables|Default|SetbClimbing true)
            (CallFunction|UpdateClimbIdlePose)
            (Class|MoverComponent|QueueNextMode _asmover_component "Flying" true)
            (Class|MoverComponent|QueueLayeredMove _asmover_component (Utilities|Struct|MakeLayeredMove_LinearVelocity (/ (- (Variables|Default|GetClimbTarget) (Transformation|GetActorLocation _returnvalue)) (Variables|Default|GetClimbDuration)) 0 "NoFlags" "OverrideAll" 255 (* (Variables|Default|GetClimbDuration) (Math|Float|MakeLiteralFloat 1e+03)) (Utilities|Struct|MakeLayeredMoveFinishVelocitySettings "0.000000,0.000000,0.000000" 0.0 "SetVelocity")))
            (Utilities|FlowControl|Delay (+ (Variables|Default|GetClimbDuration) (Math|Float|MakeLiteralFloat 0.05)))
            (Variables|Default|SetClimbExitDuration (Math|Float|Max(Float) 0.01 (/ (Math|Vector|Distance(Vector) (Transformation|GetActorLocation (Variables|Default|GetClimber)) (Variables|Default|GetClimbExitTarget)) (Math|Float|Max(Float) (Variables|Ladder|GetClimbSpeed) 1.0))))
            (Class|MoverComponent|QueueLayeredMove (Variables|Default|GetClimberMover) (Utilities|Struct|MakeLayeredMove_LinearVelocity (/ (- (Variables|Default|GetClimbExitTarget) (Transformation|GetActorLocation (Variables|Default|GetClimber))) (Variables|Default|GetClimbExitDuration)) 0 "NoFlags" "OverrideAll" 255 (* (Variables|Default|GetClimbExitDuration) (Math|Float|MakeLiteralFloat 1e+03)) (Utilities|Struct|MakeLayeredMoveFinishVelocitySettings "0.000000,0.000000,0.000000" 0.0 "SetVelocity")))
            (Utilities|FlowControl|Delay (+ (Variables|Default|GetClimbExitDuration) (Math|Float|MakeLiteralFloat 0.05)))
            (Variables|Default|SetbClimbing false)
            (CallFunction|UpdateClimbIdlePose)
            (Utilities|IsValid (Variables|Default|GetClimberMover)
              (:Is%20Valid
                (Class|MoverComponent|QueueNextMode (Variables|Default|GetClimberMover) "Falling" false))))
          (:CastFailed
            (bind _ascharacter (Utilities|Casting|CastToCharacter _returnvalue))
            (Variables|Default|SetClimbTarget (Variables|Default|GetClimbExitTarget))
            (Pawn|Components|CharacterMovement|SetMovementMode (Variables|/Script/Engine.Character|GetCharacterMovement _ascharacter) "MOVE_None" 0)
            (Variables|Default|SetbClimbing true)))))))

(fn ConstructionScript)

(fn SetLadderOccupied
  (params (bWantOccupy :type Boolean))
  (Variables|Default|SetbOccupied bWantOccupy)
  (Default|CallOnLadderOccupied))

(fn UpdateClimbIdlePose
  (bind _asskeletal_mesh_component (Utilities|Casting|CastToSkeletalMeshComponent (Actor|GetComponentbyClass (Variables|Default|GetClimber) "/Script/Engine.SkeletalMeshComponent")))
  (bind _assandbox_character_mover_abp (Utilities|Casting|CastToSandboxCharacter_Mover_ABP (Components|SkeletalMesh|GetAnimInstance _asskeletal_mesh_component)))
  (Variables|Default|SetClimbAnimInstance _assandbox_character_mover_abp)
  (Variables|/Game/Blueprints/SandboxCharacter_Mover_ABP.SandboxCharacter_Mover_ABP_C|SetLadderClimbing _assandbox_character_mover_abp (Variables|Default|GetbClimbing)))