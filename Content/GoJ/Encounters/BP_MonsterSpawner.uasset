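; BP_MonsterSpawner is an encounter spawner that places a wave of BP_Monster_Base actors around its own location.
; SpawnWave runs automatically on BeginPlay when AutoSpawnOnBeginPlay is set, creating SpawnCount monsters.
; Random X and Y offsets within SpawnRadius form a square area rather than a circle, with a fixed upward offset.
; Monsters spawn unrotated and ignore collision, with no ground or navmesh check.
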(event EventBeginPlay
  (if (Variables|Spawner|GetbAutoSpawnOnBeginPlay)
    (CallFunction|SpawnWave)))

(event Collision|EventActorBeginOverlap
  (params (OtherActor :type Actor%20Object%20Reference)))

(event EventTick
  (params (DeltaSeconds :type Float%20%28single-precision%29)))

(fn ConstructionScript)

(fn SpawnWave
  (bind _spawnradius (Variables|Spawner|GetSpawnRadius))
  (for _index (range 0 (- (Variables|Spawner|GetSpawnCount) (Class|KismetSystemLibrary|MakeLiteralInteger 1)))
    (Game|SpawnActorfromClass "/Game/GoJ/Monsters/BP_Monster_Base.BP_Monster_Base_C" (Math|Transform|MakeTransform (+ (Transformation|GetActorLocation self) (Math|Vector|MakeVector (Math|Random|RandomFloatinRange (- 0.0 _spawnradius) _spawnradius) (Math|Random|RandomFloatinRange (- 0.0 _spawnradius) _spawnradius) 1.2e+02))) "AlwaysSpawn" "MultiplyWithRoot" 0 0)))