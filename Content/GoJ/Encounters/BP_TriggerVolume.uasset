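; BP_TriggerVolume is an encounter trigger that starts spawner waves and opens doors when the player character enters it.
; On overlap it casts the actor to BP_PlayerCharacter, marks itself triggered, then calls SpawnWave on each linked spawner and SetDoorOpen(true) on each linked door.
; A TriggerOnce flag optionally limits it to a single activation.
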(event EventBeginPlay)

(event Collision|EventActorBeginOverlap
  (params (OtherActor :type Actor%20Object%20Reference))
  (if (not (and (Variables|Trigger|GetbTriggerOnce) (Variables|Default|GetbTriggered)))
    (Utilities|Casting|CastToBP_PlayerCharacter OtherActor)
    (Variables|Default|SetbTriggered true)
    (for _array_element (Variables|Trigger|GetSpawners)
      (Default|SpawnWave _array_element))
    (for _array_element_2 (Variables|Trigger|GetDoors)
      (Default|SetDoorOpen _array_element_2 true))))

(event EventTick
  (params (DeltaSeconds :type Float%20%28single-precision%29)))

(fn ConstructionScript)