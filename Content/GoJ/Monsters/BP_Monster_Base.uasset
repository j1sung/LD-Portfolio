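; BP_Monster_Base is a monster character that chases and melee-attacks the player, driven entirely from Tick.
; Within detection range it turns toward player pawn 0 and moves straight at it with movement input, without pathfinding.
; Within attack range it calls LightAttack on its AC_Combat component, gated by a game-time cooldown.
; When AC_Health reports death, it disables capsule collision, ragdolls the mesh, stops ticking and expires shortly after.
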(event EventBeginPlay)

(event Collision|EventActorBeginOverlap
  (params (OtherActor :type Actor%20Object%20Reference)))

(event EventTick
  (params (DeltaSeconds :type Float%20%28single-precision%29))
  (bind _returnvalue (Game|Player|GetPlayerPawn 0))
  (bind _self self)
  (bind _returnvalue_2 (Transformation|GetActorLocation _self))
  (bind _returnvalue_3 (Transformation|GetActorLocation _returnvalue))
  (bind _returnvalue_4 (Math|Vector|Distance(Vector) _returnvalue_2 _returnvalue_3))
  (bind _asac_health (Utilities|Casting|CastToAC_Health (Actor|GetComponentbyClass _self "/Game/GoJ/Components/AC_Health.AC_Health_C")))
  (if (Variables|/Game/GoJ/Components/AC_Health.AC_Health_C|GetbIsDead _asac_health)
    (Collision|SetCollisionEnabled (Variables|Collision|GetCapsuleComponent) "NoCollision")
    (Collision|SetCollisionProfileName (Variables|Character|GetMesh) "Ragdoll" true :!class /Script/Engine.PrimitiveComponent)
    (Physics|SetSimulatePhysics (Variables|Character|GetMesh) true)
    (Actor|Tick|SetActorTickEnabled _self)
    (Actor|SetLifeSpan _self 3.0)
    (elif (< _returnvalue_4 (Variables|Default|GetDetectionRange))
      (Transformation|SetActorRotation _self (Math|Rotator|FindLookatRotation _returnvalue_2 _returnvalue_3))
      (if (< _returnvalue_4 (Variables|Default|GetAttackRange))
        (if (> (- (Utilities|Time|GetGameTimeinSeconds) (Variables|Default|GetLastAttackTime)) (Variables|Default|GetAttackCooldown))
          (bind _asac_combat (Utilities|Casting|CastToAC_Combat (Actor|GetComponentbyClass _self "/Game/GoJ/Components/AC_Combat.AC_Combat_C")))
          (Default|LightAttack _asac_combat _returnvalue)
          (Variables|Default|SetLastAttackTime (Utilities|Time|GetGameTimeinSeconds)))
        (else
          (Pawn|Input|AddMovementInput _self (Math|Vector|Normalize (- _returnvalue_3 _returnvalue_2)) 1.0 false))))))

(fn ConstructionScript)