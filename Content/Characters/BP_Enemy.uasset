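; BP_Enemy is an enemy character Blueprint that maps Enhanced Input actions to gameplay components, with no AI logic in its graphs.
; Sprint, crouch and dodge go to Locomotion, stance toggle to Stance, and interact to Interaction.
; Light and heavy attack both call the same Combat AttackForward, and dodge passes a zero direction vector.
; BeginPlay, Tick and overlap are disabled stubs, and construction only calls the parent.
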(event Input|EnhancedActionEvents|EnhancedInputActionIA_Interact
  (params (ActionValue :type Boolean) (ElapsedSeconds :type Float%20%28double-precision%29) (TriggeredSeconds :type Float%20%28double-precision%29) (InputAction :type Input%20Action%20Object%20Reference :default "/Game/GoJ/Player/Input/IA_Interact.IA_Interact"))
  (:Started
    (Default|TryInteract (Variables|Default|GetInteraction))))

(event Input|EnhancedActionEvents|EnhancedInputActionIA_Sprint
  (params (ActionValue :type Boolean) (ElapsedSeconds :type Float%20%28double-precision%29) (TriggeredSeconds :type Float%20%28double-precision%29) (InputAction :type Input%20Action%20Object%20Reference :default "/Game/GoJ/Player/Input/IA_Sprint.IA_Sprint"))
  (bind _locomotion (Variables|Default|GetLocomotion))
  (:Started
    (Default|RequestSprint _locomotion true))
  (:Completed
    (Default|RequestSprint _locomotion false)))

(event Input|EnhancedActionEvents|EnhancedInputActionIA_Crouch
  (params (ActionValue :type Boolean) (ElapsedSeconds :type Float%20%28double-precision%29) (TriggeredSeconds :type Float%20%28double-precision%29) (InputAction :type Input%20Action%20Object%20Reference :default "/Game/GoJ/Player/Input/IA_Crouch.IA_Crouch"))
  (bind _locomotion (Variables|Default|GetLocomotion))
  (:Started
    (Default|RequestCrouch _locomotion true))
  (:Completed
    (Default|RequestCrouch _locomotion false)))

(event Input|EnhancedActionEvents|EnhancedInputActionIA_ToggleStance
  (params (ActionValue :type Boolean) (ElapsedSeconds :type Float%20%28double-precision%29) (TriggeredSeconds :type Float%20%28double-precision%29) (InputAction :type Input%20Action%20Object%20Reference :default "/Game/GoJ/Player/Input/IA_ToggleStance.IA_ToggleStance"))
  (:Started
    (Default|ToggleStance (Variables|Default|GetStance))))

(event Input|EnhancedActionEvents|EnhancedInputActionIA_Dodge
  (params (ActionValue :type Boolean) (ElapsedSeconds :type Float%20%28double-precision%29) (TriggeredSeconds :type Float%20%28double-precision%29) (InputAction :type Input%20Action%20Object%20Reference :default "/Game/GoJ/Player/Input/IA_Dodge.IA_Dodge"))
  (:Started
    (Default|RequestDodge (Variables|Default|GetLocomotion) (Math|Vector|MakeVector 0.0 0.0 0.0))))

(event Input|EnhancedActionEvents|EnhancedInputActionIA_LightAttack
  (params (ActionValue :type Boolean) (ElapsedSeconds :type Float%20%28double-precision%29) (TriggeredSeconds :type Float%20%28double-precision%29) (InputAction :type Input%20Action%20Object%20Reference :default "/Game/GoJ/Player/Input/IA_LightAttack.IA_LightAttack"))
  (:Started
    (Default|AttackForward (Variables|Default|GetCombat))))

(event Input|EnhancedActionEvents|EnhancedInputActionIA_HeavyAttack
  (params (ActionValue :type Boolean) (ElapsedSeconds :type Float%20%28double-precision%29) (TriggeredSeconds :type Float%20%28double-precision%29) (InputAction :type Input%20Action%20Object%20Reference :default "/Game/GoJ/Player/Input/IA_HeavyAttack.IA_HeavyAttack"))
  (:Started
    (Default|AttackForward (Variables|Default|GetCombat))))

(event EventBeginPlay)

(event Collision|EventActorBeginOverlap
  (params (OtherActor :type Actor%20Object%20Reference)))

(event EventTick
  (params (DeltaSeconds :type Float%20%28single-precision%29)))

(fn ConstructionScript
  (|CallParentFunction))