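; An interactable elevator actor that travels between its starting position and a fixed height above it.
; Interaction or a player character overlapping its box calls Activate, which picks the opposite end as the target unless already moving.
; Tick moves it at constant speed, snaps it within a small tolerance and flips the top/bottom state.
; CallToFloor sets separate floor variables that the movement logic never reads.
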(event OnComponentBeginOverlap(Box)
  (params (OverlappedComponent :type Primitive%20Component%20Object%20Reference) (OtherActor :type Actor%20Object%20Reference) (OtherComp :type Primitive%20Component%20Object%20Reference) (OtherBodyIndex :type Integer) (bFromSweep :type Boolean) (SweepResult :type Hit%20Result%20Structure%20%28by%20ref%29))
  (Utilities|Casting|CastToBP_PlayerCharacter OtherActor)
  (CallFunction|Activate))

(event EventBeginPlay
  (Variables|Default|SetBaseLoc (Transformation|GetActorLocation self)))

(event Collision|EventActorBeginOverlap
  (params (OtherActor :type Actor%20Object%20Reference)))

(event EventTick
  (params (DeltaSeconds :type Float%20%28single-precision%29))
  (bind _self self)
  (bind _targetloc (Variables|Default|GetTargetLoc))
  (bind _movespeed (Variables|Elevator|GetMoveSpeed))
  (bind _returnvalue (Transformation|GetActorLocation _self))
  (bind _returnvalue_2 (Math|Interpolation|VInterptoConstant _returnvalue _targetloc DeltaSeconds _movespeed))
  (if (Variables|Default|GetbMoving)
    (Transformation|SetActorLocation _self _returnvalue_2 false false)
    (if (< (Math|Vector|Distance(Vector) _returnvalue_2 (Variables|Default|GetTargetLoc)) (Math|Float|MakeLiteralFloat 2.0))
      (Transformation|SetActorLocation _self (Variables|Default|GetTargetLoc) false false)
      (Variables|Default|SetbMoving false)
      (Variables|Default|SetbAtTop (not (Variables|Default|GetbAtTop))))))

(event EventHandleInteract
  (CallFunction|Activate))

(fn ConstructionScript)

(fn CalltoFloor
  (params (Floor :type Integer))
  (Variables|Default|SetTargetFloor Floor)
  (Variables|Default|SetbIsMoving true))

(fn Activate
  (if (not (Variables|Default|GetbMoving))
    (Variables|Default|SetTargetLoc (select (Variables|Default|GetbAtTop) (Variables|Default|GetBaseLoc) (+ (Variables|Default|GetBaseLoc) (Math|Vector|MakeVector 0.0 0.0 (Variables|Elevator|GetMoveHeight)))))
    (Variables|Default|SetbMoving true)))